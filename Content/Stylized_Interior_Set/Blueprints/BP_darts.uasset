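; BP_darts is an interactive darts cabinet prop whose two doors the player opens and closes.
; Overlapping its Box enables input on the first player controller, and ending the overlap disables it.
; The select action drives a FlipFlop that alternately plays and reverses a Timeline, swinging the left and right door meshes in mirrored yaw.
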(event OnComponentBeginOverlap(Box)
  (params (OverlappedComponent :type Primitive%20Component%20Object%20Reference) (OtherActor :type Actor%20Object%20Reference) (OtherComp :type Primitive%20Component%20Object%20Reference) (OtherBodyIndex :type Integer) (bFromSweep :type Boolean) (SweepResult :type Hit%20Result%20Structure%20%28by%20ref%29))
  ;[1 1 1] enableinput
  (Input|EnableInput (Class|GameplayStatics|GetPlayerControllerfromID)))

(event OnComponentEndOverlap(Box)
  (params (OverlappedComponent :type Primitive%20Component%20Object%20Reference) (OtherActor :type Actor%20Object%20Reference) (OtherComp :type Primitive%20Component%20Object%20Reference) (OtherBodyIndex :type Integer))
  ;[1 1 1] enableinput
  (Input|DisableInput (Class|GameplayStatics|GetPlayerControllerfromID)))

(event Input|ActionEvents|InputActionselect
  (params (Key :type Key%20Structure :default "None"))
  (:Pressed
    (Utilities|FlowControl|FlipFlop
      (:A
        (bind _新建轨迹_0 (Timeline|时间轴_0 Play)
          (:Update
            (Transformation|SetRelativeRotation (Variables|Default|GetSM_darts_door_R) (Math|Rotator|MakeRotator 0.0 0.0 _新建轨迹_0) false false)
            (Transformation|SetRelativeRotation (Variables|Default|GetSM_darts_door_L) (Math|Rotator|MakeRotator 0.0 0.0 (- 1.8e+02 _新建轨迹_0)) false false))))
      (:B
        (Timeline|时间轴_0 Reverse)))))

(fn ConstructionScript)