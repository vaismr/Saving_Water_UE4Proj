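; BP_Picture_120x120 is a placeable wall picture for the hallway that picks its image texture at construction time.
; The construction script creates a dynamic material on the mesh and sets its "Picture Color" parameter from the PictureColors texture array.
; The image is either a seeded random pick or a clamped ColorID.
; An optional seed derived from the distance to world origin makes random picks depend on placement, and the event graph is unused.
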(event EventBeginPlay)

(event Collision|EventActorBeginOverlap
  (params (OtherActor :type Actor%20Object%20Reference)))

(event EventTick
  (params (DeltaSeconds :type Float%20%28single-precision%29)))

(fn ConstructionScript
  (bind _picture_colors (LocalVariables|GetPicture%20Colors))
  (bind _membervar_0 (Utilities|Struct|BreakST_Picture_120x120_Colors _picture_colors))
  (bind _returnvalue (Utilities|Array|Length _membervar_0))
  (bind _returnvalue_2 (- _returnvalue 1))
  (if (Variables|Default|GetEnable%20Random%20Seed)
    (Variables|Seed|SetInitial%20Seed (Math|Random|MakeRandomStream (Math|Float|Truncate (Math|Vector|VectorLength (Transformation|GetWorldLocation (Variables|Default|GetPicture_120x120)))))))
  (bind _returnvalue_3 (Rendering|Material|CreateDynamicMaterialInstance (Variables|Default|GetPicture_120x120) 0 (Rendering|Material|GetMaterial (Variables|Default|GetPicture_120x120) 0) "None" :!class /Script/Engine.PrimitiveComponent))
  (Rendering|Material|SetTextureParameterValue _returnvalue_3 "Picture Color" (Utilities|Array|Get(acopy) (Utilities|Struct|BreakST_Picture_120x120_Colors (LocalVariables|GetPicture%20Colors)) (select (Variables|Default|GetEnable%20Random%20Image) (Math|Random|RandomIntegerinRangefromStream 0 _returnvalue_2 (Variables|Seed|GetInitial%20Seed)) (Math|Integer|Clamp(Integer) (Variables|Default|GetColorID) 0 _returnvalue_2)))))